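; Interactable lantern pickup that gives the player a lantern and sets off a scare with a bird and a monster scream.
; Overlapping the collision shows a press-E prompt, and Interaction calls CallMonster.
; CallMonster enables the character's lantern light and destroys the pickup's components.
; Unless the character's IsSoundPlaying flag is set, it then plays sounds while the bird rises and is destroyed, holding that flag until finished.
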(event `self.Colision.OnComponentBeginOverlap`
  (params (OverlappedComponent :type "PrimitiveComponent Object Reference") (OtherActor :type "Actor Object Reference") (OtherComp :type "PrimitiveComponent Object Reference") (OtherBodyIndex :type Integer) (bFromSweep :type Boolean) (SweepResult :type "HitResult Structure (by ref)"))
  (cast `/Game/FirstPerson/Blueprints/BP_FirstPersonCharacter` OtherActor)
  (`self.EnableInput` (`GameplayStatics.GetPlayerCharacter` 0) (`GameplayStatics.GetPlayerController` 0))
  (bind _returnvalue (`|CreateWidget` "/Game/Widget/WD_PressEToInteract.WD_PressEToInteract_C"))
  (bind _output_get (set `self.WD_PressEtoInteract` _returnvalue))
  (`UserWidget.AddToViewport` _output_get 0))

(event `self.Colision.OnComponentEndOverlap`
  (params (OverlappedComponent :type "PrimitiveComponent Object Reference") (OtherActor :type "Actor Object Reference") (OtherComp :type "PrimitiveComponent Object Reference") (OtherBodyIndex :type Integer))
  (cast `/Game/FirstPerson/Blueprints/BP_FirstPersonCharacter` OtherActor)
  (bind _foundwidgets (`WidgetBlueprintLibrary.GetAllWidgetsOfClass` "/Game/Widget/WD_PressEToInteract.WD_PressEToInteract_C"))
  (`Widget.RemoveFromParent` _foundwidgets))

(event `CallMonster`
  (bind _monsterscream (`self.MonsterScream`))
  (bind _asbp_first_person_character (cast `/Game/FirstPerson/Blueprints/BP_FirstPersonCharacter` (`GameplayStatics.GetPlayerPawn` 0)))
  (set `/Game/FirstPerson/Blueprints/BP_FirstPersonCharacter.GotLantern?` true _asbp_first_person_character)
  (`SceneComponent.SetHiddenInGame` (`/Game/FirstPerson/Blueprints/BP_FirstPersonCharacter.LanternLightCharacter` _asbp_first_person_character) false false)
  (`ActorComponent.K2_DestroyComponent` (`self.LanternLight`))
  (`ActorComponent.K2_DestroyComponent` (`self.Colision`))
  (`ActorComponent.K2_DestroyComponent` (`self.LanternBody`))
  (if (not (`/Game/FirstPerson/Blueprints/BP_FirstPersonCharacter.IsSoundPlaying` _asbp_first_person_character))
    (set `/Game/FirstPerson/Blueprints/BP_FirstPersonCharacter.IsSoundPlaying` true _asbp_first_person_character)
    (`GameplayStatics.PlaySound2D` (`self.SoundMade`) 1.0 1.0 0.0 null null)
    (`KismetSystemLibrary.MoveComponentTo` (`self.Bird`) (0.0 0.0 300.0) (struct) false false 2.0)
    (`GameplayStatics.PlaySound2D` (`self.SoundMade`) 1.0 1.0 0.0 null null)
    (`KismetSystemLibrary.Delay` 2.0)
    (`GameplayStatics.PlaySound2D` _monsterscream 1.0 1.0 0.0 null null)
    (`KismetSystemLibrary.MoveComponentTo` (`self.Bird`) (0.0 0.0 1000.0) (struct) false false 2.0)
    (`ActorComponent.K2_DestroyComponent` (`self.Bird`))
    (`KismetSystemLibrary.Delay` (+ (`SoundBase.Duration` _monsterscream) 1.0))
    (set `/Game/FirstPerson/Blueprints/BP_FirstPersonCharacter.IsSoundPlaying` false _asbp_first_person_character)))

(fn `Interaction`
  (returns (HasInteracted :type Boolean))
  (`self.CallMonster`)
  (return true))

(fn `UserConstructionScript`)