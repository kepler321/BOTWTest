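; Scripted Korok encounter in which a Korok steals a gem when the player walks into its trigger.
; The actor stays hidden and non-colliding until Tick sees the player's HasTalkedToKorok flag.
; The trigger runs chained MoveComponentTo steps to grab the gem, carry it through goal points and destroy it, then sets KorokStole and shows timed dialogue.
; A separate KorokDeath overlap shows its own dialogue, then removes itself.
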(event `self.ReceiveBeginPlay`
  (`self.SetActorHiddenInGame` true)
  (`PrimitiveComponent.SetCollisionEnabled` (`self.KorokDeath`) "NoCollision")
  (`PrimitiveComponent.SetCollisionEnabled` (`self.Trigger`) "NoCollision"))

(event `self.ReceiveTick`
  (params (DeltaSeconds :type "Float (single-precision)"))
  (bind _asbp_first_person_character (cast `/Game/FirstPerson/Blueprints/BP_FirstPersonCharacter` (`GameplayStatics.GetPlayerPawn` 0)))
  (if (`/Game/FirstPerson/Blueprints/BP_FirstPersonCharacter.HasTalkedToKorok?` _asbp_first_person_character)
    (`/Engine/EditorBlueprintResources/StandardMacros.DoOnce` false
      (:`Completed`
        (`PrimitiveComponent.SetCollisionEnabled` (`self.KorokDeath`) "QueryOnly")
        (`PrimitiveComponent.SetCollisionEnabled` (`self.Trigger`) "QueryOnly")
        (`self.SetActorHiddenInGame` false)))))

(event `self.Trigger.OnComponentBeginOverlap`
  (params (OverlappedComponent :type "PrimitiveComponent Object Reference") (OtherActor :type "Actor Object Reference") (OtherComp :type "PrimitiveComponent Object Reference") (OtherBodyIndex :type Integer) (bFromSweep :type Boolean) (SweepResult :type "HitResult Structure (by ref)"))
  (bind _korok (`self.Korok`))
  (bind _relativelocation (`SceneComponent.RelativeLocation` (`self.GoalLast`)))
  (cast `/Game/FirstPerson/Blueprints/BP_FirstPersonCharacter` OtherActor)
  (`KismetSystemLibrary.MoveComponentTo` (`self.Korok`) (- (`SceneComponent.RelativeLocation` (`self.Gem`)) (0.0 0.0 -30.0)) (struct) true false 1.0)
  (`ActorComponent.K2_DestroyComponent` (`self.Trigger`))
  (`KismetSystemLibrary.Delay` 0.5)
  (`SceneComponent.K2_AttachToComponent` (`self.Gem`) (`self.Korok attach`) "None" "SnapToTarget" "SnapToTarget" "KeepWorld" true)
  (`KismetSystemLibrary.MoveComponentTo` (`self.Korok`) (`SceneComponent.RelativeLocation` (`self.Goal1`)) (struct) false false 0.5)
  (`KismetSystemLibrary.MoveComponentTo` (`self.Korok`) (`SceneComponent.RelativeLocation` (`self.Goal2`)) (struct) false false 0.5)
  (`KismetSystemLibrary.MoveComponentTo` _korok _relativelocation (struct) false false 2.0)
  (`KismetSystemLibrary.MoveComponentTo` _korok _relativelocation (struct :`Roll` 90.0) false false 0.1)
  (`ActorComponent.K2_DestroyComponent` (`self.Gem`))
  (set `self.Korok Stole` true)
  (`self.UI`
    (:`then`
      _)
    (:`else`
      (bind _returnvalue (`|CreateWidget` "/Game/Widget/WD_KorokTalk.WD_KorokTalk_C" (`GameplayStatics.GetPlayerController` 0)))
      (bind _output_get (set `self.UI` _returnvalue))))
  (`UserWidget.AddToViewport` _output_get 0)
  (`TextBlock.SetText` (`/Game/Widget/WD_KorokTalk.Talk` (`self.UI`)) (`KismetTextLibrary.Conv_StringToText` (`self.KorokStealText`)))
  (`KismetSystemLibrary.Delay` 4.0)
  (bind _foundwidgets (`WidgetBlueprintLibrary.GetAllWidgetsOfClass` "/Game/Widget/WD_KorokTalk.WD_KorokTalk_C"))
  (`Widget.RemoveFromParent` _foundwidgets))

(event `self.KorokDeath.OnComponentBeginOverlap`
  (params (OverlappedComponent :type "PrimitiveComponent Object Reference") (OtherActor :type "Actor Object Reference") (OtherComp :type "PrimitiveComponent Object Reference") (OtherBodyIndex :type Integer) (bFromSweep :type Boolean) (SweepResult :type "HitResult Structure (by ref)"))
  (cast `/Game/FirstPerson/Blueprints/BP_FirstPersonCharacter` OtherActor)
  (`self.UI2`
    (:`then`
      _)
    (:`else`
      (bind _returnvalue (`|CreateWidget` "/Game/Widget/WD_KorokTalk.WD_KorokTalk_C" (`GameplayStatics.GetPlayerController` 0)))
      (bind _output_get (set `self.UI2` _returnvalue))))
  (`UserWidget.AddToViewport` _output_get 0)
  (`TextBlock.SetText` (`/Game/Widget/WD_KorokTalk.Talk` (`self.UI2`)) (`KismetTextLibrary.Conv_StringToText` (`self.KorokDeathText`)))
  (`KismetSystemLibrary.Delay` 4.0)
  (bind _foundwidgets (`WidgetBlueprintLibrary.GetAllWidgetsOfClass` "/Game/Widget/WD_KorokTalk.WD_KorokTalk_C"))
  (`Widget.RemoveFromParent` _foundwidgets)
  (`ActorComponent.K2_DestroyComponent` (`self.KorokDeath`)))

(fn `UserConstructionScript`)