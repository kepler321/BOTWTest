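; Altar actor where the player places the red, yellow and blue gems, triggering the "Calamity Is Back" event.
; Overlap toggles input and the interact prompt once the Korok has been talked to; interacting reveals each gem the player holds.
; Tick polls gem visibility as placement state and fires once when all show.
; It plays a monster cutscene, then screams, spawns an NPC AI, shows dialogue and sets the player's CanEscape.
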(event `self.ReceiveTick`
  (params (DeltaSeconds :type "Float (single-precision)"))
  (bind _returnvalue (`GameplayStatics.GetPlayerController` 0))
  (bind _returnvalue_2 (`GameplayStatics.GetPlayerController` 0))
  (bind _returnvalue_3 (`GameplayStatics.GetPlayerPawn` 0))
  ;[1 1 1] Play Sound If all Gems are on table and play cutscene
  (if (and (`SceneComponent.bVisible` (`self.RedGem`)) (`SceneComponent.bVisible` (`self.YellowGem`)) (`SceneComponent.bVisible` (`self.BlueGem`)))
    (`/Engine/EditorBlueprintResources/StandardMacros.DoOnce` false
      (:`Completed`
        (`self.DisableInput` _returnvalue_3 _returnvalue_2)
        (`PlayerController.SetViewTargetWithBlend` _returnvalue_2 (`self.CameraReference`) 2.0 "VTBlend_Linear" 0.0 false)
        (`SceneComponent.SetHiddenInGame` (`self.Monster`) false false)
        (`SceneComponent.SetHiddenInGame` (`self.Eye1`) false false)
        (`SceneComponent.SetHiddenInGame` (`self.Eye`) false false)
        (bind (_outactor _returnvalue_4) (`LevelSequencePlayer.CreateLevelSequencePlayer` "/Game/Sequencers/CalamityIsBack.CalamityIsBack"))
        (`MovieSceneSequencePlayer.Play` _returnvalue_4)
        (`KismetSystemLibrary.Delay` 8.0)
        (`PlayerController.SetViewTargetWithBlend` _returnvalue (`GameplayStatics.GetPlayerCharacter` 0) 2.0 "VTBlend_Linear" 0.0 false)
        (`KismetSystemLibrary.Delay` 2.0)
        (`self.EnableInput` _returnvalue_3 _returnvalue)
        (`GameplayStatics.PlaySound2D` "/Game/Sounds/Monster/NazgulScream_Cue.NazgulScream_Cue" 1.0 1.0 0.0 null null)
        (`AIBlueprintHelperLibrary.SpawnAIFromClass` "/Game/BluePrints/AI/NPC/BP_NPC.BP_NPC_C" "/Game/BluePrints/AI/NPC/BT_NPC.BT_NPC" (`SceneComponent.K2_GetComponentLocation` (`self.AISpawn`)) (struct) false null)
        (`ActorComponent.K2_DestroyComponent` (`self.Monster`))
        (`ActorComponent.K2_DestroyComponent` (`self.Eye`))
        (`ActorComponent.K2_DestroyComponent` (`self.Eye1`))
        (`self.UI`
          (:`then`
            _)
          (:`else`
            (bind _returnvalue_5 (`|CreateWidget` "/Game/Widget/WD_KorokTalk.WD_KorokTalk_C" (`GameplayStatics.GetPlayerController` 0)))
            (bind _output_get (set `self.UI` _returnvalue_5))))
        (`UserWidget.AddToViewport` _output_get 0)
        (`TextBlock.SetText` (`/Game/Widget/WD_KorokTalk.Talk` (`self.UI`)) (`KismetTextLibrary.Conv_StringToText` (`self.Calamity is back text`)))
        (`KismetSystemLibrary.Delay` 4.0)
        (bind _foundwidgets (`WidgetBlueprintLibrary.GetAllWidgetsOfClass` "/Game/Widget/WD_KorokTalk.WD_KorokTalk_C"))
        (`Widget.RemoveFromParent` _foundwidgets)
        (bind _asbp_first_person_character (cast `/Game/FirstPerson/Blueprints/BP_FirstPersonCharacter` (`GameplayStatics.GetPlayerPawn` 0)))
        (set `/Game/FirstPerson/Blueprints/BP_FirstPersonCharacter.CanEscape` true _asbp_first_person_character)))))

(event `InputAction|Interaction`
  (params (Key :type "Key Structure"))
  ;[1 1 1] Toggle The Lights on altar on if interacter and alredy got the Rupie
  (:`Pressed`
    (bind _asbp_first_person_character (cast `/Game/FirstPerson/Blueprints/BP_FirstPersonCharacter` (`GameplayStatics.GetPlayerPawn` 0)))
    (`|ExecutionSequence`
      (:`then_0`
        (if (`/Game/FirstPerson/Blueprints/BP_FirstPersonCharacter.GotYellowGem` _asbp_first_person_character)
          (`SceneComponent.SetVisibility` (`self.YellowGem`) true false)
          (bind _foundwidgets (`WidgetBlueprintLibrary.GetAllWidgetsOfClass` "/Game/Widget/WD_PressEToInteract.WD_PressEToInteract_C"))
          (`Widget.RemoveFromParent` _foundwidgets)))
      (:`then_1`
        (if (`/Game/FirstPerson/Blueprints/BP_FirstPersonCharacter.GotRedGem` _asbp_first_person_character)
          (`SceneComponent.SetVisibility` (`self.RedGem`) true false)
          (bind _foundwidgets_2 (`WidgetBlueprintLibrary.GetAllWidgetsOfClass` "/Game/Widget/WD_PressEToInteract.WD_PressEToInteract_C"))
          (`Widget.RemoveFromParent` _foundwidgets_2)))
      (:`then_2`
        (if (`/Game/FirstPerson/Blueprints/BP_FirstPersonCharacter.GotBlueGem` _asbp_first_person_character)
          (`SceneComponent.SetVisibility` (`self.BlueGem`) true false)
          (bind _foundwidgets_3 (`WidgetBlueprintLibrary.GetAllWidgetsOfClass` "/Game/Widget/WD_PressEToInteract.WD_PressEToInteract_C"))
          (`Widget.RemoveFromParent` _foundwidgets_3))))))

(event `self.ReceiveActorBeginOverlap`
  (params (OtherActor :type "Actor Object Reference"))
  (bind _returnvalue (`GameplayStatics.GetPlayerController` 0))
  ;[1 1 1] Widget To Interact
  (bind _asbp_first_person_character (cast `/Game/FirstPerson/Blueprints/BP_FirstPersonCharacter` (`GameplayStatics.GetPlayerPawn` 0)))
  (if (and (`SceneComponent.bVisible` (`self.RedGem`)) (`SceneComponent.bVisible` (`self.YellowGem`)) (`SceneComponent.bVisible` (`self.BlueGem`)))
    (`self.DisableInput` _returnvalue :!label _label)
    (bind _foundwidgets (`WidgetBlueprintLibrary.GetAllWidgetsOfClass` "/Game/Widget/WD_PressEToInteract.WD_PressEToInteract_C"))
    (`Widget.RemoveFromParent` _foundwidgets)
    (elif (`/Game/FirstPerson/Blueprints/BP_FirstPersonCharacter.HasTalkedToKorok?` _asbp_first_person_character)
      (`self.EnableInput` _returnvalue)
      (bind _returnvalue_2 (`|CreateWidget` "/Game/Widget/WD_PressEToInteract.WD_PressEToInteract_C"))
      (`UserWidget.AddToViewport` _returnvalue_2 0))))

(event `self.ReceiveActorEndOverlap`
  (params (OtherActor :type "Actor Object Reference"))
  ;[1 1 1] Widget To Interact
  (cast `/Game/FirstPerson/Blueprints/BP_FirstPersonCharacter` (`GameplayStatics.GetPlayerPawn` 0))
  (goto _label))

(fn `UserConstructionScript`)