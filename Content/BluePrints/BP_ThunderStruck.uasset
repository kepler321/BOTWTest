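; BP_ThunderStruck is an actor that plays a one-time thunder and lightning effect once the player has the yellow gem.
; Tick polls GotYellowGem on the first-person character, with a DoOnce gate limiting the effect to a single run.
; It plays a 2D thunder sound and flickers the ThunderStruck component's intensity between random bright values and zero through short delays, then destroys itself.
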(event `self.ReceiveTick`
  (params (DeltaSeconds :type "Float (single-precision)"))
  (bind _returnvalue (`KismetMathLibrary.RandomFloatInRange` 1000.0 3000.0))
  (bind _thunderstruck (`self.ThunderStruck`))
  (bind _asbp_first_person_character (cast `/Game/FirstPerson/Blueprints/BP_FirstPersonCharacter` (`GameplayStatics.GetPlayerPawn` 0)))
  (if (`/Game/FirstPerson/Blueprints/BP_FirstPersonCharacter.GotYellowGem` _asbp_first_person_character)
    (`/Engine/EditorBlueprintResources/StandardMacros.DoOnce` false
      (:`Completed`
        (`GameplayStatics.PlaySound2D` "/Game/Sounds/SFX_Thunder_Cue.SFX_Thunder_Cue" 1.0 1.0 0.0 null null)
        (`LightComponent.SetIntensity` _thunderstruck _returnvalue)
        (`KismetSystemLibrary.Delay` 0.4)
        (`LightComponent.SetIntensity` _thunderstruck 0.0)
        (`KismetSystemLibrary.Delay` 0.1)
        (`LightComponent.SetIntensity` _thunderstruck _returnvalue)
        (`KismetSystemLibrary.Delay` 0.3)
        (`LightComponent.SetIntensity` _thunderstruck 0.0)
        (`KismetSystemLibrary.Delay` 0.1)
        (`LightComponent.SetIntensity` _thunderstruck _returnvalue)
        (`KismetSystemLibrary.Delay` 0.2)
        (`self.K2_DestroyActor`)))))

(fn `UserConstructionScript`)