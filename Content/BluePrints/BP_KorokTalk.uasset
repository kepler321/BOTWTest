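; BP_KorokTalk is a one-time trigger actor that lets the player talk to a Korok through stepped dialogue.
; Overlap shows an interact prompt and enables input, while leaving removes the dialogue widget and disables input.
; Each Interaction press stops walking and advances the Dialog array in WD_KorokTalk, with a talk sound played only once.
; Reaching the end restores walk speed, sets HasTalkedToKorok on the player character and destroys the trigger.
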(event `self.ReceiveActorBeginOverlap`
  (params (OtherActor :type "Actor Object Reference"))
  ;[1 1 1] Creation of Widget and Enable/Disable Input
  (bind _returnvalue (`|CreateWidget` "/Game/Widget/WD_PressEToInteract.WD_PressEToInteract_C"))
  (`UserWidget.AddToViewport` _returnvalue 0)
  (`self.EnableInput` (`GameplayStatics.GetPlayerController` 0)))

(event `self.ReceiveActorEndOverlap`
  (params (OtherActor :type "Actor Object Reference"))
  ;[1 1 1] Creation of Widget and Enable/Disable Input
  (bind _foundwidgets (`WidgetBlueprintLibrary.GetAllWidgetsOfClass` "/Game/Widget/WD_KorokTalk.WD_KorokTalk_C"))
  (`Widget.RemoveFromParent` _foundwidgets)
  (`self.DisableInput` (`GameplayStatics.GetPlayerController` 0)))

(event `InputAction|Interaction`
  (params (Key :type "Key Structure"))
  ;[1 1 1] Talk to Korok and Destroy Trigger
  (:`Pressed`
    (bind _asbp_first_person_character (cast `/Game/FirstPerson/Blueprints/BP_FirstPersonCharacter` (`GameplayStatics.GetPlayerPawn` 0)))
    (bind _charactermovement (`Character.CharacterMovement` _asbp_first_person_character))
    (set `CharacterMovementComponent.MaxWalkSpeed` 0.0 _charactermovement)
    (bind _foundwidgets (`WidgetBlueprintLibrary.GetAllWidgetsOfClass` "/Game/Widget/WD_PressEToInteract.WD_PressEToInteract_C"))
    (`Widget.RemoveFromParent` _foundwidgets)
    (if (not (`self.DidSoundPlay`))
      (`GameplayStatics.PlaySound2D` (`self.KorokTalk`) 1.0 1.0 0.0 null null)
      (set `self.DidSoundPlay` true))
    (`/Engine/EditorBlueprintResources/StandardMacros.IncrementInt` (`self.TalkIndex`)
      (:`  `
        (if (<= (`self.TalkIndex`) (`KismetArrayLibrary.Array_Length` (`self.Dialog`)))
          (`self.UI`
            (:`then`
              _)
            (:`else`
              (bind _returnvalue (`|CreateWidget` "/Game/Widget/WD_KorokTalk.WD_KorokTalk_C" (`GameplayStatics.GetPlayerController` 0)))
              (bind _output_get (set `self.UI` _returnvalue))
              (`UserWidget.AddToViewport` _output_get 0)))
          (`TextBlock.SetText` (`/Game/Widget/WD_KorokTalk.Talk` (`self.UI`)) (`KismetTextLibrary.Conv_StringToText` (`|GetArrayItem` (`self.Dialog`) (`self.TalkIndex`))))
          (if (== (`self.TalkIndex`) (`KismetArrayLibrary.Array_Length` (`self.Dialog`)))
            (bind _foundwidgets_2 (`WidgetBlueprintLibrary.GetAllWidgetsOfClass` "/Game/Widget/WD_KorokTalk.WD_KorokTalk_C"))
            (`Widget.RemoveFromParent` _foundwidgets_2)
            (set `CharacterMovementComponent.MaxWalkSpeed` 400.0 _charactermovement)
            (set `/Game/FirstPerson/Blueprints/BP_FirstPersonCharacter.HasTalkedToKorok?` true _asbp_first_person_character)
            (`self.K2_DestroyActor`)))))))

(fn `UserConstructionScript`)