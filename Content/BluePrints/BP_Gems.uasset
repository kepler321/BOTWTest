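; BP_Gems is a collectible gem whose Material sets both its look and which colour flag it grants the player.
; It starts hidden, and Tick reveals it once the player has talked to the Korok, keeping the red gem hidden unless the referenced BP_KorokStealGem has stolen.
; Overlapping a visible gem enables input and shows a prompt; Interaction destroys it and updates the player's gem count.
; Korok dialogue popup chains are unconnected.
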(event `self.ReceiveTick`
  (params (DeltaSeconds :type "Float (single-precision)"))
  (bind _returnvalue (== (`self.Material`) "/Game/Materials/MI_RedGem.MI_RedGem"))
  (bind _asbp_first_person_character (cast `/Game/FirstPerson/Blueprints/BP_FirstPersonCharacter` (`GameplayStatics.GetPlayerPawn` 0)))
  (if (`/Game/FirstPerson/Blueprints/BP_FirstPersonCharacter.HasTalkedToKorok?` _asbp_first_person_character)
    (`self.SetActorHiddenInGame` false)
    (bind _asbp_korok_steal_gem (cast `/Game/BluePrints/BP_KorokStealGem` (`self.ActorReference`)))
    (if (`/Game/BluePrints/BP_KorokStealGem.Korok Stole` _asbp_korok_steal_gem)
      (if _returnvalue
        (`self.SetActorHiddenInGame` false))
      (elif _returnvalue
        (`self.SetActorHiddenInGame` true)))))

(event `self.ReceiveBeginPlay`
  (`self.SetActorHiddenInGame` true))

(event `InputAction|Interaction`
  (params (Key :type "Key Structure"))
  (:`Pressed`
    (bind _asbp_first_person_character (cast `/Game/FirstPerson/Blueprints/BP_FirstPersonCharacter` (`GameplayStatics.GetPlayerPawn` 0)))
    (`self.K2_DestroyActor`)
    (set `/Game/FirstPerson/Blueprints/BP_FirstPersonCharacter.GemsGot` (+ 1 (`/Game/FirstPerson/Blueprints/BP_FirstPersonCharacter.GemsGot` _asbp_first_person_character)) _asbp_first_person_character)
    (if (== (`self.Material`) "/Game/Materials/MI_BlueGem.MI_BlueGem")
      (set `/Game/FirstPerson/Blueprints/BP_FirstPersonCharacter.GotBlueGem` true _asbp_first_person_character)
      (elif (== (`self.Material`) "/Game/Materials/MI_YellowGem.MI_YellowGem")
        (set `/Game/FirstPerson/Blueprints/BP_FirstPersonCharacter.GotYellowGem` true _asbp_first_person_character)
        (elif (== (`self.Material`) "/Game/Materials/MI_RedGem.MI_RedGem")
          (set `/Game/FirstPerson/Blueprints/BP_FirstPersonCharacter.GotRedGem` true _asbp_first_person_character))))))

(event `self.ReceiveActorBeginOverlap`
  (params (OtherActor :type "Actor Object Reference"))
  (cast `/Game/FirstPerson/Blueprints/BP_FirstPersonCharacter` (`GameplayStatics.GetPlayerPawn` 0))
  (if (not (`self.bHidden`))
    (`self.EnableInput` (`GameplayStatics.GetPlayerController` 0))
    (bind _returnvalue (`|CreateWidget` (`self.InteractionWD`)))
    (`UserWidget.AddToViewport` _returnvalue 0)))

(event `self.ReceiveActorEndOverlap`
  (params (OtherActor :type "Actor Object Reference"))
  (cast `/Game/FirstPerson/Blueprints/BP_FirstPersonCharacter` (`GameplayStatics.GetPlayerPawn` 0))
  (`self.DisableInput` (`GameplayStatics.GetPlayerController` 0))
  (bind _foundwidgets (`WidgetBlueprintLibrary.GetAllWidgetsOfClass` (`self.InteractionWD`)))
  (`Widget.RemoveFromParent` _foundwidgets))

(fn `UserConstructionScript`
  (`PrimitiveComponent.SetMaterial` (`self.Gem`) 0 (`self.Material`)))